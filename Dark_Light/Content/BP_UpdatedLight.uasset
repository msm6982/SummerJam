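; Light cube for a top-down light puzzle: basic cubes start lit, while other cubes can be grabbed and carried by the player.
; When cubes' collision spheres begin or end overlapping, a recursive search from the basic cubes relights chained neighbours and switches off unreached ones.
; Switching swaps the material and sets spot and point light intensity.
; Player entry and exit report light or dark, with one-time or repeating dialogue.
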(event `self.ReceiveBeginPlay`
  ;[1 1 1] Begin Play
  (if (not (`KismetSystemLibrary.IsValid` (`self.Player`)))
    (bind _asbp_light_game_top_down (cast `/Game/BP_LightGameTopDown` (`GameplayStatics.GetPlayerPawn` 0)))
    (bind _output_get (set `self.Player` _asbp_light_game_top_down)))
  (`KismetSystemLibrary.PrintString` (`KismetSystemLibrary.GetDisplayName` _output_get))
  (bind _outactors (`GameplayStatics.GetAllActorsOfClass` "BP_UpdatedLight_C"))
  (bind _output_get_2 (set `self.AllCubes` _outactors))
  (for _array_element _output_get_2
    (if (`/Game/BP_UpdatedLight.isBasicCube` _array_element)
      (`KismetArrayLibrary.Array_AddUnique` (`self.BasicCubes`) _array_element)
      (`KismetArrayLibrary.Array_AddUnique` (`self.CurrentlyLitCubes`) _array_element)
      (else
        (`KismetArrayLibrary.Array_AddUnique` (`self.LightCubes`) _array_element))))
  (bind _output_get_3 (set `self.OtherCubes` _output_get_2))
  (bind _returnvalue (`KismetArrayLibrary.Array_RemoveItem` _output_get_3 self))
  (`KismetSystemLibrary.PrintString` (`KismetStringLibrary.Conv_BoolToString` _returnvalue)))

(event `self.ReceiveActorBeginOverlap`
  (params (OtherActor :type "Actor Object Reference"))
  (bind _player (`self.Player`))
  ;[1 1 1] Overlap with player, start dialogue
  (if (== OtherActor _player)
    (bind _returnvalue (`/Game/BP_LightGameTopDown.AlreadyInLight` _player))
    (if _returnvalue
      _
      (elif (not (`self.DoneOnce`))
        (set `self.DoneOnce` true)
        (`/Game/BP_LightGameTopDown.LightOverlap` (`self.Player`) (`self.PlayerLightDialogue`) :!label _label)
        (elif (`self.Repeat`)
          (goto _label)
          (else
            (`/Game/BP_LightGameTopDown.LightOverlap` (`self.Player`) (`self.Empty`))))))))

(event `self.ReceiveActorEndOverlap`
  (params (OtherActor :type "Actor Object Reference"))
  (bind _player (`self.Player`))
  ;[1 1 1] End Overlap
  (if (== OtherActor _player)
    (bind _returnvalue (`/Game/BP_LightGameTopDown.IsInLight` _player))
    (if _returnvalue
      _
      (elif (not (`self.DoneOnce`))
        (set `self.DoneOnce` true)
        (`/Game/BP_LightGameTopDown.DarkOverlap` (`self.Player`) (`self.PlayerDarkDialogue`) :!label _label_2)
        (elif (`self.Repeat`)
          (goto _label_2)
          (else
            (`/Game/BP_LightGameTopDown.DarkOverlap` (`self.Player`) (`self.Empty`))))))))

(event `EV_LightOn`
  ;[1 1 1] Turn Light On/Off
  (set `self.activated` true)
  (`PrimitiveComponent.SetMaterial` (`self.Cube`) 0 (`|GetArrayItem` (`self.matArray`)))
  (`LightComponent.SetIntensity` (`self.SpotLight`) (`self.spotLightIntensity`))
  (`LightComponent.SetIntensity` (`self.PointLight`) (`self.PointLightIntensity`)))

(event `EV_LightOff`
  ;[1 1 1] Turn Light On/Off
  (set `self.activated` false)
  (`PrimitiveComponent.SetMaterial` (`self.Cube`) 0 (`|GetArrayItem` (`self.matArray`) 1))
  (`LightComponent.SetIntensity` (`self.SpotLight`) 0.0)
  (`LightComponent.SetIntensity` (`self.PointLight`) 0.0))

(event `self.BoxCollider.OnComponentBeginOverlap`
  (params (OverlappedComponent :type "PrimitiveComponent Object Reference") (OtherActor :type "Actor Object Reference") (OtherComp :type "PrimitiveComponent Object Reference") (OtherBodyIndex :type Integer) (bFromSweep :type Boolean) (SweepResult :type "HitResult Structure (by ref)"))
  ;[1 1 1] Toggle Grabbability
  (`|ExecutionSequence`
    (:`then_0`
      (if (and (== (`self.Player`) OtherActor) (not (`self.isBasicCube`)))
        (set `/Game/BP_LightGameTopDown.detectedCube` self (`self.Player`))
        (set `self.grabable` true)))))

(event `self.BoxCollider.OnComponentEndOverlap`
  (params (OverlappedComponent :type "PrimitiveComponent Object Reference") (OtherActor :type "Actor Object Reference") (OtherComp :type "PrimitiveComponent Object Reference") (OtherBodyIndex :type Integer))
  ;[1 1 1] Toggle Grabbability
  (`|ExecutionSequence`
    (:`then_0`
      (if (and (== (`self.Player`) OtherActor) (not (`self.isBasicCube`)))
        (set `/Game/BP_LightGameTopDown.detectedCube` null (`self.Player`))
        (set `self.grabable` false)))))

(event `self.CollisionSphere.OnComponentBeginOverlap`
  (params (OverlappedComponent :type "PrimitiveComponent Object Reference") (OtherActor :type "Actor Object Reference") (OtherComp :type "PrimitiveComponent Object Reference") (OtherBodyIndex :type Integer) (bFromSweep :type Boolean) (SweepResult :type "HitResult Structure (by ref)"))
  (cast `/Game/BP_UpdatedLight` OtherActor)
  (bind _output_get (set `self.CurrentlyLitCubes` (`self.BasicCubes`)))
  (for _array_element (`self.AllCubes`)
    (`KismetArrayLibrary.Array_Clear` (`/Game/BP_UpdatedLight.CheckedOverlaps` _array_element)))
  (`self.RecursiveSearchChainCubes` _output_get)
  (for _array_element_2 (`self.LightCubes`)
    (if (== (`KismetArrayLibrary.Array_Find` (`self.CurrentlyLitCubes`) _array_element_2) -1)
      (`self.EV_LightOff` _array_element_2))))

(event `self.CollisionSphere.OnComponentEndOverlap`
  (params (OverlappedComponent :type "PrimitiveComponent Object Reference") (OtherActor :type "Actor Object Reference") (OtherComp :type "PrimitiveComponent Object Reference") (OtherBodyIndex :type Integer))
  (cast `/Game/BP_UpdatedLight` OtherActor)
  (bind _output_get (set `self.CurrentlyLitCubes` (`self.BasicCubes`)))
  (for _array_element (`self.AllCubes`)
    (`KismetArrayLibrary.Array_Clear` (`/Game/BP_UpdatedLight.CheckedOverlaps` _array_element)))
  (`self.RecursiveSearchChainCubes` _output_get)
  (for _array_element_2 (`self.LightCubes`)
    (if (== (`KismetArrayLibrary.Array_Find` (`self.CurrentlyLitCubes`) _array_element_2) -1)
      (`self.EV_LightOff` _array_element_2))))

(event `EV_GrabCube`
  (if (`self.grabable`)
    (`PrimitiveComponent.SetCollisionResponseToChannel` (`self.Cube`) "ECC_Pawn" "ECR_Overlap")
    (`self.K2_AttachToComponent` (`/Game/BP_LightGameTopDown.holdSpot` (`self.Player`)) "center" "SnapToTarget" "SnapToTarget" "KeepWorld")))

(fn `ChainCubes`
  (locals (LitUpCubes :type "Array of /Game/BP_UpdatedLight Object Reference"))
  (for _array_element (`self.LightCubes`)
    (bind _collisionsphere (`/Game/BP_UpdatedLight.CollisionSphere` _array_element))
    (for _array_element_2 (`PrimitiveComponent.GetOverlappingActors` _collisionsphere "BP_UpdatedLight_C")
      (bind _asbp_updated_light (cast `/Game/BP_UpdatedLight` _array_element_2))
      (if (`PrimitiveComponent.IsOverlappingComponent` _collisionsphere (`/Game/BP_UpdatedLight.CollisionSphere` _asbp_updated_light))
        (`self.EV_LightOn` _asbp_updated_light)))))

(fn `CheckIfConnectedToBaseCube`)

(fn `CheckIfInDark`
  (returns (InLight :type Boolean) (BaseConnectionPresent :type Boolean))
  (locals (ReturnVal :type Boolean :default true) (ReturnBaseConnection :type Boolean :default true))
  (for _array_element (`self.OtherCubes`)
    (if (`PrimitiveComponent.IsOverlappingComponent` (`/Game/BP_UpdatedLight.CollisionSphere` _array_element) (`self.CollisionSphere`))
      (if (or (`/Game/BP_UpdatedLight.activated` _array_element) (`/Game/BP_UpdatedLight.isBasicCube` _array_element))
        (set `local.ReturnVal` false)
        (set `local.ReturnBaseConnection` false))))
  (return (`local.ReturnVal`) false))

(fn `CheckIfInLight`
  (returns (Return :type Boolean) (ConnectedToBase :type Boolean))
  (locals (ReturnVal :type Boolean) (ConnectionToBase :type Boolean))
  (for _array_element (`self.OtherCubes`)
    (if (`/Game/BP_UpdatedLight.activated` _array_element)
      (if (`PrimitiveComponent.IsOverlappingComponent` (`/Game/BP_UpdatedLight.CollisionSphere` _array_element) (`self.CollisionSphere`))
        (set `local.ReturnVal` true)
        (if (`/Game/BP_UpdatedLight.isBasicCube` _array_element)
          (set `local.ConnectionToBase` true)))))
  (return (`local.ReturnVal`) (`local.ConnectionToBase`)))

(fn `RecursiveSearchChainCubes`
  (params (RecursiveCubes :type "Array of Actor Object Reference"))
  (locals (ParentRecursion :type "/Game/BP_UpdatedLight Object Reference") (ChildRecursion :type "/Game/BP_UpdatedLight Object Reference") (OverlappingActors :type "Array of Actor Object Reference") (ComponetTest :type "Array of PrimitiveComponent Object Reference"))
  (for _array_element RecursiveCubes
    (bind _asbp_updated_light (cast `/Game/BP_UpdatedLight` _array_element))
    (bind _output_get (set `local.ParentRecursion` _asbp_updated_light))
    (set `local.OverlappingActors` (`PrimitiveComponent.GetOverlappingActors` (`/Game/BP_UpdatedLight.CollisionSphere` _output_get) "BP_UpdatedLight_C"))
    (for _array_element_2 (`local.OverlappingActors`)
      (bind _asbp_updated_light_2 (cast `/Game/BP_UpdatedLight` _array_element_2))
      (bind _output_get_2 (set `local.ChildRecursion` _asbp_updated_light_2))
      (if (!= _output_get_2 (`local.ParentRecursion`))
        (if (`PrimitiveComponent.IsOverlappingComponent` (`/Game/BP_UpdatedLight.CollisionSphere` (`local.ParentRecursion`)) (`/Game/BP_UpdatedLight.CollisionSphere` (`local.ChildRecursion`)))
          (`self.EV_LightOn` (`local.ChildRecursion`))
          (`KismetArrayLibrary.Array_AddUnique` (`self.CurrentlyLitCubes`) (`local.ChildRecursion`)))
        (`KismetArrayLibrary.Array_AddUnique` (`/Game/BP_UpdatedLight.CheckedOverlaps` (`local.ChildRecursion`)) (`local.ParentRecursion`))
        (`KismetArrayLibrary.Array_AddUnique` (`/Game/BP_UpdatedLight.CheckedOverlaps` (`local.ParentRecursion`)) (`local.ChildRecursion`))))
    (if (not (<= (`KismetArrayLibrary.Array_Length` (`/Game/BP_UpdatedLight.CheckedOverlaps` (`local.ParentRecursion`))) (`KismetArrayLibrary.Array_Length` (`local.OverlappingActors`))))
      (`self.RecursiveSearchChainCubes` (`local.OverlappingActors`))))
  (return))

(fn `UserConstructionScript`
  (if (`self.isBasicCube`)
    (`self.EV_LightOn`)
    (else
      (`self.EV_LightOff`))))