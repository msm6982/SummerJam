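; BP_ExitWithTrigger is a level exit door that opens for an activated light and wins the level on entry.
; On BeginPlay it shifts itself to a random Y offset.
; An activated BP_UpdatedLight overlapping the sensor collision triggers a timeline that lerps the Sphere component upward as the door.
; When BP_LightGameTopDown overlaps the entry collision, a completion event prints a win message.
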(event `self.ReceiveBeginPlay`
  (`self.K2_AddActorWorldOffset` (`KismetMathLibrary.MakeVector` 0.0 (`KismetMathLibrary.RandomFloatInRange` 250.0 3200.0))))

(event `EV_OpenDoors`
  (bind (_direction _alpha) (`Timeline|TL_liftTheDoor`)
    (:`Update`
      (`SceneComponent.K2_SetRelativeLocation` (`self.Sphere`) (`KismetMathLibrary.MakeVector` 0.0 0.0 (`KismetMathLibrary.Lerp` 0.0 250.0 _alpha)) false false))))

(event `self.Collision Door Senser.OnComponentBeginOverlap`
  (params (OverlappedComponent :type "PrimitiveComponent Object Reference") (OtherActor :type "Actor Object Reference") (OtherComp :type "PrimitiveComponent Object Reference") (OtherBodyIndex :type Integer) (bFromSweep :type Boolean) (SweepResult :type "HitResult Structure (by ref)"))
  (bind _asbp_updated_light (cast `/Game/BP_UpdatedLight` OtherActor))
  (if (`/Game/BP_UpdatedLight.activated` _asbp_updated_light)
    (`self.EV_OpenDoors`)))

(event `self.Collision_door_entry.OnComponentBeginOverlap`
  (params (OverlappedComponent :type "PrimitiveComponent Object Reference") (OtherActor :type "Actor Object Reference") (OtherComp :type "PrimitiveComponent Object Reference") (OtherBodyIndex :type Integer) (bFromSweep :type Boolean) (SweepResult :type "HitResult Structure (by ref)"))
  (cast `/Game/BP_LightGameTopDown` OtherActor)
  (`self.EV_CompleteLevel`))

(event `EV_CompleteLevel`
  (`KismetSystemLibrary.PrintString` "You Win!"))

(fn `UserConstructionScript`)